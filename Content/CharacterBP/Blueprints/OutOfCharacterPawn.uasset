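; OutOfCharacterPawn is a free-moving pawn with an orthographic camera, panned and zoomed by player input.
; Move axes offset the Box with sweep in the X-Z plane, so panning respects collision.
; Zoom actions step a clamped Magnification value, which Tick applies to the camera's ortho width.
; On possession it caches the GTController, through which the C key toggles the control panel's character box.
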(event `self.ReceiveTick`
  (params (DeltaSeconds :type "Float (single-precision)"))
  (`self.UpdateCamera`))

(event `Setup`
  (params (`GT Controller` :type "Controller Object Reference"))
  ;[1 1 1] Initialisation
  (set `self.OwningController` (cast `/Game/CharacterBP/Blueprints/GTController` `GT Controller` :!pure true)))

(event `self.ReceivePossessed`
  (params (NewController :type "Controller Object Reference"))
  ;[1 1 1] Initialisation
  (`self.Setup` NewController))

(event `UpdateCamera`
  ;[1 1 1] Update Camera Tick
  (`CameraComponent.SetOrthoWidth` (`self.Camera`) (* 1024.0 (`self.Magnification`))))

(event `Key|C`
  (params (Key :type "Key Structure"))
  ;[1 1 1] Open Character Panel
  (:`Pressed`
    (`/Game/UI/ControlPanel.ToggleCharacterBox` (`/Game/CharacterBP/Blueprints/GTController.ControlPanelRef` (`self.OwningController`)))))

(event `InputAction|ZoomIn`
  (params (Key :type "Key Structure"))
  ;[1 1 1] Camera Zoom
  (:`Pressed`
    (set `self.Magnification` (`KismetMathLibrary.FClamp` (+ (`self.Magnification`) -0.2) 0.1 10.0))))

(event `InputAxis|MoveUp`
  (params (AxisValue :type "Float (single-precision)"))
  (`SceneComponent.K2_AddWorldOffset` (`self.Box`) (* (0.0 0.0 10.0) AxisValue) true false))

(event `InputAction|ZoomOut`
  (params (Key :type "Key Structure"))
  ;[1 1 1] Camera Zoom
  (:`Pressed`
    (set `self.Magnification` (`KismetMathLibrary.FClamp` (+ (`self.Magnification`) 0.2) 0.1 10.0))))

(event `InputAxis|MoveRight`
  (params (AxisValue :type "Float (single-precision)"))
  (`SceneComponent.K2_AddWorldOffset` (`self.Box`) (* (10.0 0.0 0.0) AxisValue) true false))

(fn `UserConstructionScript`)